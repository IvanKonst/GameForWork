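; BP_BlackboxPawn is a testing-tool pawn meant to show a skill-choice HUD during clash sequences.
; Two handlers toggle the WBP_BlackboxDecider widget, mouse cursor and UI/game input mode when skill buttons are drawn or the first sequence finishes.
; The setup that creates the widget, spawns BP_BlackboxEvents and binds those handlers is disconnected, and BeginPlay is empty, so none of it currently runs.
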(event Custom|ClashSequenceDrawSkillButtons_Event_0
  (bind _returnvalue (Game|GetPlayerController 0))
  ;[1 1 1] Listen in on the clash sequence events and display the HUD to choose a skill for the following sequence
  (Widget|SetVisibility (Variables|Default|GetWidgetChoiceSelector) "Visible")
  (Input|SetInputModeUIOnly _returnvalue 0 "DoNotLock")
  (Variables|/Script/Engine.PlayerController|SetbShowMouseCursor _returnvalue true))

(event Custom|ClashSequenceFirstSequenceFinished_Event_0
  (bind _returnvalue (Game|GetPlayerController 0))
  ;[1 1 1] Listen in on the clash sequence events and display the HUD to choose a skill for the following sequence
  (Widget|SetVisibility (Variables|Default|GetWidgetChoiceSelector) "Hidden")
  (Input|SetInputModeGameOnly _returnvalue)
  (Variables|/Script/Engine.PlayerController|SetbShowMouseCursor _returnvalue false))

(event EventBeginPlay)

(fn ConstructionScript)