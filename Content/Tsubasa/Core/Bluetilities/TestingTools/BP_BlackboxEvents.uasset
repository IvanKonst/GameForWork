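; Testing actor that plays Level Sequences as singles, pairs, arrays or skill-choice clashes, mostly reporting completion through event dispatchers.
; Clashes play an opening sequence, signal skill buttons, then play the chosen or default follow-up when a timer expires or a decision interrupts it.
; Arrays chain through finish callbacks, using pause playback settings at a chosen index and a timer to resume.
; Leftover callback and print-timer experiments sit in the EventGraph.
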(event Custom|printEvent
  ;[1 1 1] Weird ass testing events
  (Development|PrintString "Hello" true true "(R=0.000000,G=0.660000,B=1.000000,A=1.000000)" 1.0))

(event Custom|StartEvent_Event
  ;[1 1 1] Weird ass testing events
  (bind _returnvalue (Utilities|Time|SetTimerbyEvent (delegate Custom|printEvent) 0.5 true))
  (Variables|Default|Settimer _returnvalue))

(event Custom|CompleteEvent_Event
  ;[1 1 1] Weird ass testing events
  (Utilities|Time|ClearandInvalidateTimerbyHandle (Variables|Default|Gettimer))
  (Default|CallEventDone))

(event Custom|StartCallBackEvent
  ;[1 1 1] Weird ass testing events
)

(event EventBeginPlay
  ;[1 1 1] Weird ass testing events
)

(event Custom|ClashSequenceWithChoiceSkillFollowUp
  (params (SequenceOne :type Level%20Sequence%20Object%20Reference) (ChoiceWaitTimer :type Float%20%28single-precision%29))
  ;[1 1 1] Clash sequence
  (bind (_outactor _returnvalue) (Sequencer|Player|CreateLevelSequencePlayer SequenceOne (Utilities|Struct|MakeMovieSceneSequencePlaybackSettings true "(Value=0)" 1.0 0.0 false false false false false false false true)))
  (Variables|Default|SetClashSeqActorOne _outactor)
  (bind _returnvalue_2 (Utilities|Time|SetTimerbyEvent (delegate Custom|OnClashSeqOneFinished) (+ (/ (Math|Conversions|ToFloat(Integer) (Utilities|Struct|BreakFrameNumber (.Frame (Utilities|TimeManagement|BreakQualifiedFrameTime (Media|MediaPlayer|GetDuration _returnvalue))))) (Math|Conversions|ToFloat(Integer) (.Numerator (Class|KismetMathLibrary|BreakFrameRate (.FrameRate (Utilities|TimeManagement|BreakQualifiedFrameTime (Media|MediaPlayer|GetDuration _returnvalue))))))) ChoiceWaitTimer)))
  (Variables|Default|SetTimerSequenceDecider _returnvalue_2)
  (Utilities|FlowControl|Delay (/ (Math|Conversions|ToFloat(Integer) (Utilities|Struct|BreakFrameNumber (.Frame (Utilities|TimeManagement|BreakQualifiedFrameTime (Media|MediaPlayer|GetDuration _returnvalue))))) (Math|Conversions|ToFloat(Integer) (.Numerator (Class|KismetMathLibrary|BreakFrameRate (.FrameRate (Utilities|TimeManagement|BreakQualifiedFrameTime (Media|MediaPlayer|GetDuration _returnvalue))))))))
  ;;[1 1 1] Setup the 2nd sequence in case there's no selected sequence i.e. default case
  (Variables|Default|SetSelectedSequenceTwoClash (Variables|Default|GetDefaultSequenceTwoClash))
  (Development|PrintString (Utilities|String|Append (Utilities|String|ToString(Float) ChoiceWaitTimer) " second(s) timer for a choice."))
  (Variables|Default|SetbClashOneDone true)
  (Default|CallClashSequenceDrawSkillButtons))

(event Custom|OnClashSeqOneFinished
  ;[1 1 1] Ability sequence
  (if (Variables|Default|GetbClashOneDone)
    (Default|CallClashSequenceFirstSequenceFinished)
    (Sequencer|Player|Stop (stale Custom|ClashSequenceWithChoiceSkillFollowUp _returnvalue) :!class /Script/MovieScene.MovieSceneSequencePlayer)
    (bind (_outactor _returnvalue) (Sequencer|Player|CreateLevelSequencePlayer (Variables|Default|GetSelectedSequenceTwoClash)))
    (Variables|Default|SetClashSeqActorTwo _outactor)
    (Sequencer|Player|Play _returnvalue :!class /Script/MovieScene.MovieSceneSequencePlayer)
    (EventDispatchers|AssignOnFinished _returnvalue (delegate Custom|OnClashSequencesFinished))))

(event Custom|OnClashSequencesFinished
  ;[1 1 1] Whole clash sequence event is done
  (Default|CallClashSequencewithChoiceSkillFollowUpFinished)
  ;[1 1 1] reset
  (Variables|Default|SetbClashOneDone false)
  ;[1 1 1] Clean up sequence actors
  (Actor|DestroyActor (Variables|Default|GetClashSeqActorOne))
  (Actor|DestroyActor (Variables|Default|GetClashSeqActorTwo)))

(event Custom|TakeDecidingAction
  (params (SelectedSequenceTwoClash :type Level%20Sequence%20Object%20Reference))
  ;[1 1 1] Interupt X second timer and go on with a selected action
  (Utilities|Time|ClearandInvalidateTimerbyHandle (Variables|Default|GetTimerSequenceDecider))
  (CallFunction|SetSequenceChoiceClashTwo SelectedSequenceTwoClash)
  (CallFunction|OnClashSeqOneFinished)
  (Development|PrintString (Utilities|String|Append "=== Taking deciding action before the " (Utilities|String|ToString(Float) (stale Custom|ClashSequenceWithChoiceSkillFollowUp ChoiceWaitTimer)) " second period ended. ===")))

(event Custom|SetSequenceChoiceClashTwo
  (params (SelectedSequenceTwoClash :type Level%20Sequence%20Object%20Reference))
  ;[1 1 1] Clash sequence
  (Variables|Default|SetSelectedSequenceTwoClash SelectedSequenceTwoClash))

(event Custom|SingleSequence
  (params (LevelSequence :type Level%20Sequence%20Object%20Reference))
  (bind (_outactor _returnvalue) (Sequencer|Player|CreateLevelSequencePlayer LevelSequence))
  (Sequencer|Player|Play _returnvalue :!class /Script/MovieScene.MovieSceneSequencePlayer)
  (EventDispatchers|BindEventtoOnFinished _returnvalue (delegate Custom|SingleFinished)))

(event Custom|SingleFinished
  (Actor|DestroyActor (stale Custom|SingleSequence _outactor))
  (Default|CallSingleSequenceFinished))

(event Custom|DoubleSequence
  (params (Sequence%20One :type Level%20Sequence%20Object%20Reference) (Sequence%20Two :type Level%20Sequence%20Object%20Reference))
  (bind (_outactor _returnvalue) (Sequencer|Player|CreateLevelSequencePlayer Sequence%20One))
  (Sequencer|Player|Play _returnvalue :!class /Script/MovieScene.MovieSceneSequencePlayer)
  (EventDispatchers|BindEventtoOnFinished _returnvalue (delegate Custom|DoubleSequenceTwo)))

(event Custom|DoubleSequenceTwo
  (Actor|DestroyActor (stale Custom|DoubleSequence _outactor))
  (bind (_outactor _returnvalue) (Sequencer|Player|CreateLevelSequencePlayer (stale Custom|DoubleSequence Sequence%20Two)))
  (Sequencer|Player|Play _returnvalue :!class /Script/MovieScene.MovieSceneSequencePlayer)
  (EventDispatchers|AssignOnFinished _returnvalue (delegate Custom|DoubleSequenceDone)))

(event Custom|DoubleSequenceDone
  (Actor|DestroyActor (stale Custom|DoubleSequenceTwo _outactor))
  (Default|CallDoubleSequenceFinished))

(event Custom|PlaySeqArr
  (params (Sequences :type Array%20of%20Level%20Sequence%20Object%20References) (PauseAtSeq :type Boolean) (SeqToPause :type Integer))
  (Variables|Default|Setcount (Utilities|Array|Length Sequences))
  (if (not (< (Variables|Default|GetcurrentIndex) (Variables|Default|Getcount)))
    (Variables|Default|Setcount 0)
    (Variables|Default|SetcurrentIndex 0)
    (Variables|Default|SetCurrentMovieSettings (Variables|Default|GetDefaultMovieSettings))
    (else
      (bind _returnvalue (Utilities|PlaySequence (Variables|Default|GetcurrentIndex) SeqToPause PauseAtSeq Sequences))
      (Utilities|IncrementIndex)
      (EventDispatchers|BindEventtoOnFinished _returnvalue (delegate Custom|CallBackSeqArr))
      (EventDispatchers|BindEventtoOnPause _returnvalue (delegate Custom|OnPause_Event_0)))))

(event Custom|CallBackSeqArr
  (Utilities|HandOffPause (- (Variables|Default|GetcurrentIndex) 1) (stale Custom|PlaySeqArr SeqToPause) (stale Custom|PlaySeqArr PauseAtSeq)
    (:true
      (CallFunction|PlaySeqArr (stale Custom|PlaySeqArr Sequences) (stale Custom|PlaySeqArr PauseAtSeq) (stale Custom|PlaySeqArr SeqToPause))
      (Development|PrintString "Playing next sequence if available." true false "(R=1.000000,G=0.112445,B=0.000000,A=1.000000)" 0.5))))

(event Custom|CreateTimer
  (params (TimerLenght :type Integer))
  (bind _returnvalue (Utilities|Time|SetTimerbyEvent (delegate Custom|EndTimer) (Math|Conversions|ToFloat(Integer) TimerLenght)))
  (Variables|Default|SetTimerHandle _returnvalue)
  (Development|PrintString "Created the timer."))

(event Custom|EndTimer
  (Utilities|Time|ClearandInvalidateTimerbyHandle (Variables|Default|GetTimerHandle))
  (Sequencer|Player|Stop (stale Custom|PlaySeqArr _returnvalue) :!class /Script/MovieScene.MovieSceneSequencePlayer)
  (CallFunction|PlaySeqArr (stale Custom|PlaySeqArr Sequences) (stale Custom|PlaySeqArr PauseAtSeq) (stale Custom|PlaySeqArr SeqToPause)))

(event Custom|OnPause_Event_0
  (CallFunction|CreateTimer 10))

(fn ConstructionScript)