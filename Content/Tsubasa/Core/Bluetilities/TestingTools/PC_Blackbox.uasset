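; PC_Blackbox is a test player controller that drives BP_BlackboxEvents, a harness for events and clash sequences with player choices.
; Number keys 1–6 trigger start, complete and callback events, a chained choice sequence, a deciding action and a single sequence.
; Clash-sequence handlers toggle the WBP_BlackboxDecider widget, cursor and input mode.
; The chains that spawn the Blackbox, create the widget and bind those handlers are disconnected, and BeginPlay is empty.
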(event Custom|eventdone_evt
  (Development|PrintString "Event done."))

(event Custom|ClashSequenceDrawSkillButtons_Event_0
  (Widget|SetVisibility (Variables|Default|GetWidgetChoiceSelector) "Visible")
  (Input|SetInputModeUIOnly self 0 "DoNotLock")
  (Variables|Default|SetbShowMouseCursor true))

(event Custom|ClashSequenceFirstSequenceFinished_Event_0
  (Widget|SetVisibility (Variables|Default|GetWidgetChoiceSelector) "Hidden")
  (Input|SetInputModeGameOnly self)
  (Variables|Default|SetbShowMouseCursor false))

(event EventBeginPlay)

(event Input|KeyboardEvents|1
  (params (Key :type Key%20Structure :default "None"))
  (:Pressed
    (Default|CallStartEvent (Variables|Default|Getblackbox))))

(event Input|KeyboardEvents|2
  (params (Key :type Key%20Structure :default "None"))
  (:Pressed
    (Default|CallCompleteEvent (Variables|Default|Getblackbox))))

(event Input|KeyboardEvents|3
  (params (Key :type Key%20Structure :default "None"))
  (:Pressed
    (Development|PrintString "Starting CallBackEvent.")
    (Default|StartCallBackEvent (Variables|Default|Getblackbox))))

(event Input|KeyboardEvents|4
  (params (Key :type Key%20Structure :default "None"))
  (:Pressed
    (CallFunction|Startsequences)))

(event Input|KeyboardEvents|5
  (params (Key :type Key%20Structure :default "None"))
  (:Pressed
    (Default|TakeDecidingAction (Variables|Default|Getblackbox) "/Game/Tsubasa/Core/Bluetilities/TestingTools/TestSequences/BlackBoxSequenceTwoChoice.BlackBoxSequenceTwoChoice")))

(event Input|KeyboardEvents|6
  (params (Key :type Key%20Structure :default "None"))
  (:Pressed
    (Default|SingleSequence (Variables|Default|Getblackbox) "/Game/Tsubasa/Core/Bluetilities/TestingTools/TestSequences/BlackBoxSequenceTwoChoice.BlackBoxSequenceTwoChoice")))

(event Custom|startsequences
  (bind _blackbox (Variables|Default|Getblackbox))
  (Development|PrintString "Sequences started.")
  (EventDispatchers|AssignClashSequencewithChoiceSkillFollowUpFinished _blackbox (delegate Custom|SequenceOneAndTwoDone_Event_0))
  (Default|ClashSequencewithChoiceSkillFollowUp _blackbox "/Game/Tsubasa/Core/Bluetilities/TestingTools/TestSequences/BlackBoxSequenceOne.BlackBoxSequenceOne" 1e+01))

(event Custom|SequenceOneAndTwoDone_Event_0
  (Development|PrintString "Sequences completed."))

(fn ConstructionScript)