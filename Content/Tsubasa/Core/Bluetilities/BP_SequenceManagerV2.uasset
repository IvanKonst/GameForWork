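; Manager that plays Level Sequence cutscenes for the football game's clashes and goal attempts, plus generic single, double and array sequences.
; Clashes play an opening sequence, show a timed skill-choice widget, then play the selected follow-up when picked or timed out.
; Forward shots chain kick, ball-flight and goalie sequences through a callback-driven array player, while other roles skip to the goalie.
; Dispatchers signal completion, and most flows toggle the master HUD.
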(event Custom|ClearSimpleAttackCooldown)

(event Custom|SimpleAttackCooldown
  (bind _returnvalue (Utilities|Time|SetTimerbyEvent (delegate Custom|ClearSimpleAttackCooldown) 1.0))
  (Variables|Timers|SetSimpleAttackHandle _returnvalue))

(event EventBeginPlay
  (Utilities|FlowControl|Sequence
    (:then_0
      ;[1 1 1] setup defaults
      (CallFunction|SetDefaultValuesScoreGoal)
      (CallFunction|SetDefaultValuesClashSequence))
    (:then_1
      ;[1 1 1] create the choice widget to be called and used
      (CallFunction|CreateChoiceWidget)
      (bind _returnvalue (Actor|GetActorOfClass "/Game/Tsubasa/Core/Blueprints/Characters/BP_Spectator.BP_Spectator_C"))
      (Variables|Default|SetSpectator _returnvalue))))

(event Custom|ClashSequenceWithChoiceSkillFollowUp
  (params (TeamTag :type Name) (ChoiceWaitTimer :type Float%20%28single-precision%29) (AttackerWonClash :type Boolean))
  (Variables|Local|SetChoiceWaitTimer ChoiceWaitTimer)
  (Utilities|FlowControl|Sequence
    (:then_0
      ;[1 1 1] Comment
      (bind _sequence (CallFunction|GetClashSequence TeamTag))
      (Utilities|IsValid _sequence
        (:Is%20Valid
          (Variables|Local|SetClashSeqOneIn _sequence))
        (:Is%20Not%20Valid
          (Development|PrintString "Invalid clash sequence one.")))
      (CallFunction|HidePlayMenu))
    (:then_1
      (bind (_outactor _returnvalue) (Sequencer|Player|CreateLevelSequencePlayer "/Game/Cinematics/Sequences/AnimationStateSequence/Characters_StateClash_02.Characters_StateClash_02" (Utilities|Struct|MakeMovieSceneSequencePlaybackSettings true "(Value=0)" 1.0 0.0 false false false false false false false true)))
      (Utilities|FlowControl|Sequence
        (:then_0
          (Variables|Local|SetClashSeqActorOne _outactor))
        (:then_1
          (bind _output_get (Variables|Default|SetClashLevelSequencerOne _returnvalue))
          (Sequencer|Player|Play _output_get :!class /Script/MovieScene.MovieSceneSequencePlayer))
        (:then_2
          (Variables|Default|SetSequenceLength (Utilities|GetLengthSeconds (Variables|Default|GetClashLevelSequencerOne))))))
    (:then_2
      (bind _returnvalue_2 (Utilities|Time|SetTimerbyEvent (delegate Custom|OnClashSeqOneFinished) (+ (Variables|Local|GetChoiceWaitTimer) (Variables|Default|GetSequenceLength)) false (Variables|Default|GetSequenceLength)))
      (Variables|Default|SetTimerSequenceDecider _returnvalue_2)
      (Utilities|Time|SetTimerbyEvent (delegate Custom|ShowChoiceWidgetEvent) (Variables|Default|GetSequenceLength)))))

(event Custom|OnClashSeqOneFinished
  ;[1 1 1] Ability sequence
  (if (Variables|Default|GetbClashOneDone)
    (Default|CallClashSequenceFirstSequenceFinished)
    (CallFunction|HideChoiceWidget)
    (Sequencer|Player|Stop (Variables|Default|GetClashLevelSequencerOne) :!class /Script/MovieScene.MovieSceneSequencePlayer)
    (bind (_outactor _returnvalue) (Sequencer|Player|CreateLevelSequencePlayer (Variables|Local|GetSelectedSequenceTwoClash)))
    (Variables|Default|SetClashLevelSequencerTwo _returnvalue)
    (Variables|Local|SetClashSeqActorTwo _outactor)
    (Sequencer|Player|Play (Variables|Default|GetClashLevelSequencerTwo) :!class /Script/MovieScene.MovieSceneSequencePlayer)
    (EventDispatchers|AssignOnFinished (Variables|Default|GetClashLevelSequencerTwo) (delegate Custom|OnClashSequencesFinished))))

(event Custom|OnClashSequencesFinished
  ;[1 1 1] Whole clash sequence event is done
  (Default|CallClashSequencewithChoiceSkillFollowUpFinished)
  ;[1 1 1] Reset bool check
  (Variables|Default|SetbClashOneDone false)
  ;[1 1 1] Clean up sequence actors
  (Actor|DestroyActor (Variables|Local|GetClashSeqActorOne))
  (Actor|DestroyActor (Variables|Local|GetClashSeqActorTwo))
  (CallFunction|ShowPlayMenu))

(event Custom|TakeDecidingAction
  (params (SelectedSequenceTwoClash :type Level%20Sequence%20Object%20Reference))
  ;[1 1 1] Interupt X second timer and go on with a selected action
  (Utilities|Time|ClearandInvalidateTimerbyHandle (Variables|Default|GetTimerSequenceDecider))
  (CallFunction|SetSeqChoiceClash2 SelectedSequenceTwoClash)
  (CallFunction|OnClashSeqOneFinished)
  (Development|PrintString (Utilities|String|Append "=== Taking deciding action before the " (Utilities|String|ToString(Float) (Variables|Local|GetChoiceWaitTimer)) " second period ended. ==="))
  (CallFunction|HideChoiceWidget))

(event Custom|ShowChoiceWidgetEvent
  (Development|PrintString (Utilities|String|Append (Utilities|String|ToString(Float) (Variables|Local|GetChoiceWaitTimer)) " second(s) timer for a choice."))
  (Variables|Default|SetbClashOneDone true)
  (CallFunction|ShowChoiceWidget))

(event Custom|SingleSequence
  (params (LevelSequence :type Level%20Sequence%20Object%20Reference) (KeepHUDHidden :type Boolean))
  (Default|HideMasterHUD (Variables|Default|GetMenuHUD))
  (bind (_outactor _returnvalue) (Sequencer|Player|CreateLevelSequencePlayer LevelSequence))
  (Sequencer|Player|Play _returnvalue :!class /Script/MovieScene.MovieSceneSequencePlayer)
  (EventDispatchers|BindEventtoOnFinished _returnvalue (delegate Custom|SingleFinished)))

(event Custom|SingleFinished
  (if (stale Custom|SingleSequence KeepHUDHidden)
    _
    (else
      (Default|ShowMasterHUD (Variables|Default|GetMenuHUD))))
  (Default|CallSingleSequenceFinished)
  (Utilities|IsValid (stale Custom|SingleSequence _outactor)
    (:Is%20Valid
      (Actor|DestroyActor (stale Custom|SingleSequence _outactor)))))

(event Custom|DoubleSequence
  (params (Sequence%20One :type Level%20Sequence%20Object%20Reference) (Sequence%20Two :type Level%20Sequence%20Object%20Reference))
  (bind (_outactor _returnvalue) (Sequencer|Player|CreateLevelSequencePlayer Sequence%20One))
  (Sequencer|Player|Play _returnvalue :!class /Script/MovieScene.MovieSceneSequencePlayer)
  (EventDispatchers|BindEventtoOnFinished _returnvalue (delegate Custom|DoubleSequenceTwo)))

(event Custom|DoubleSequenceTwo
  (Actor|DestroyActor (stale Custom|DoubleSequence _outactor))
  (bind (_outactor _returnvalue) (Sequencer|Player|CreateLevelSequencePlayer (stale Custom|DoubleSequence Sequence%20Two)))
  (Sequencer|Player|Play _returnvalue :!class /Script/MovieScene.MovieSceneSequencePlayer)
  (EventDispatchers|AssignOnFinished _returnvalue (delegate Custom|DoubleSequenceDone)))

(event Custom|DoubleSequenceDone
  (Actor|DestroyActor (stale Custom|DoubleSequenceTwo _outactor))
  (Default|CallDoubleSequenceFinished))

(event Custom|ScoreGoalSequence
  (params (SuccessfulScore :type Boolean) (KeepHUDHidden :type Boolean) (AttackerRole :type EPlayerRole%20Enum :default "forward"))
  (Variables|Local|SetGoalieBallSequenceTF (select SuccessfulScore (Variables|Defaultvalues|GetDefaultGoalieMissedBallSequence) (Variables|Defaultvalues|GetDefaultGoalieCatchBallSequence)))
  (Default|HideMasterHUD (Variables|Default|GetMenuHUD))
  (switch Utilities|FlowControl|Switch|SwitchonEPlayerRole AttackerRole
    (:forward
      (CallFunction|PlaySeqArr (Utilities|Array|MakeArray (Variables|Defaultvalues|GetDefaultKickGoalSequence) "/Game/Cinematics/Sequences/BallSequence/FlyingBall_01.FlyingBall_01" (Variables|Local|GetGoalieBallSequenceTF)) false)
      (EventDispatchers|BindEventtoArrSeqFinished (delegate Custom|ArrSeqFinished_Event)))
    (:midfield
      (CallFunction|KickSequenceFinished :!label _label))
    (:defender
      (goto _label))
    (:goalkeeper
      (goto _label))))

(event Custom|KickSequenceFinished
  (if true
    (Variables|Local|SetGoalieBallSequenceTF (Variables|Defaultvalues|GetDefaultGoalieMissedBallSequence))
    (else
      (Variables|Local|SetGoalieBallSequenceTF (Variables|Defaultvalues|GetDefaultGoalieCatchBallSequence))))
  (bind (_outactor _returnvalue) (Sequencer|Player|CreateLevelSequencePlayer (Variables|Local|GetGoalieBallSequenceTF)))
  (Sequencer|Player|Play _returnvalue :!class /Script/MovieScene.MovieSceneSequencePlayer)
  (EventDispatchers|BindEventtoOnFinished _returnvalue (delegate Custom|ScoreGoalEventFinished))
  (if (Utilities|IsValid 0)
    (Actor|DestroyActor 0)
    (Default|CallScoreGoalKickSequenceFinished)))

(event Custom|ArrSeqFinished_Event
  (if (stale Custom|ScoreGoalSequence KeepHUDHidden)
    _
    (else
      (Default|ShowMasterHUD (Variables|Default|GetMenuHUD))))
  (CallFunction|SetDefaultValuesScoreGoal)
  (Default|CallScoreGoalFinished))

(event Custom|ScoreGoalEventFinished
  (if true
    _
    (else
      (Default|ShowMasterHUD (Variables|Default|GetMenuHUD))))
  (Actor|DestroyActor (stale Custom|KickSequenceFinished _outactor))
  (CallFunction|SetDefaultValuesScoreGoal)
  (Default|CallScoreGoalFinished))

(event Custom|SetGoalieSequences
  (params (GoalieMissedBallSequence :type Level%20Sequence%20Object%20Reference) (GoaliesCatchBallSequence :type Level%20Sequence%20Object%20Reference))
  (Variables|Local|SetGoalieMissedBallSequence GoalieMissedBallSequence)
  (Variables|Local|SetGoaliesCatchBallSequence GoaliesCatchBallSequence))

(event Custom|SetKickSequence
  (params (KickGoalSequence :type Level%20Sequence%20Object%20Reference))
  (Variables|Local|SetKickGoalSequence KickGoalSequence))

(event Custom|SetDefaultValuesScoreGoal
  (Variables|Local|SetKickGoalSequence (Variables|Defaultvalues|GetDefaultKickGoalSequence))
  (Variables|Local|SetGoalieMissedBallSequence (Variables|Defaultvalues|GetDefaultGoalieMissedBallSequence))
  (Variables|Local|SetGoaliesCatchBallSequence (Variables|Defaultvalues|GetDefaultGoalieCatchBallSequence)))

(event Custom|CreateChoiceWidget
  (bind _returnvalue (UserInterface|CreateWidget "/Game/Tsubasa/UI/Widgets/WBP_ChoiceMenu.WBP_ChoiceMenu_C"))
  (bind _output_get (Variables|Default|SetWidget_ChoiceMenu _returnvalue))
  (UserInterface|Viewport|AddtoViewport _output_get 0)
  (Widget|SetVisibility _output_get "Hidden")
  (EventDispatchers|BindEventtoClashSequenceDrawSkillButtons (delegate Custom|ShowChoiceWidget))
  (EventDispatchers|BindEventtoClashSequenceFirstSequenceFinished (delegate Custom|HideChoiceWidget)))

(event Custom|ShowChoiceWidget
  (bind _returnvalue (Game|GetPlayerController 0))
  (Widget|SetVisibility (Variables|Default|GetWidget_ChoiceMenu) "Visible")
  (Input|SetInputModeUIOnly _returnvalue 0 "DoNotLock")
  (Variables|/Script/Engine.PlayerController|SetbShowMouseCursor _returnvalue true)
  (Development|PrintString "ChoiceMenu shown." true false "(R=1.000000,G=0.027115,B=0.000000,A=1.000000)"))

(event Custom|HideChoiceWidget
  (bind _returnvalue (Game|GetPlayerController 0))
  (Widget|SetVisibility (Variables|Default|GetWidget_ChoiceMenu) "Hidden")
  (Input|SetInputModeUIOnly _returnvalue 0 "DoNotLock")
  (Variables|/Script/Engine.PlayerController|SetbShowMouseCursor _returnvalue true)
  (Development|PrintString "ChoiceMenu hidden." true false "(R=1.000000,G=0.027115,B=0.000000,A=1.000000)"))

(event Custom|PlaySeqArr
  (params (Sequences :type Array%20of%20Level%20Sequence%20Object%20References) (PauseAtSeq :type Boolean) (SeqToPause :type Integer))
  (Variables|MultiSeqVariables|Setcount (Utilities|Array|Length Sequences))
  (if (not (< (Variables|MultiSeqVariables|GetcurrentIndex) (Variables|MultiSeqVariables|Getcount)))
    (Variables|MultiSeqVariables|Setcount 0)
    (Variables|MultiSeqVariables|SetcurrentIndex 0)
    (Default|CallArrSeqFinished)
    (else
      (bind _returnvalue (Utilities|CreateLevelSequence Sequences (Variables|MultiSeqVariables|GetcurrentIndex) SeqToPause PauseAtSeq))
      (Utilities|IncrementSeqArrIndex)
      (EventDispatchers|BindEventtoOnFinished _returnvalue (delegate Custom|CallBackSeqArr))
      (EventDispatchers|BindEventtoOnPause _returnvalue (delegate Custom|OnPause_Event_0)))))

(event Custom|CallBackSeqArr
  (CallFunction|PlaySeqArr (stale Custom|PlaySeqArr Sequences) (stale Custom|PlaySeqArr PauseAtSeq) (stale Custom|PlaySeqArr SeqToPause))
  (Development|PrintString "Playing next sequence if available." true false "(R=1.000000,G=0.112445,B=0.000000,A=1.000000)" 0.5))

(event Custom|CreateTimer
  (params (TimerLenght :type Integer))
  (bind _returnvalue (Utilities|Time|SetTimerbyEvent (delegate Custom|EndTimer) (Math|Conversions|ToFloat(Integer) TimerLenght)))
  (Variables|Timers|SetTimerHandle _returnvalue))

(event Custom|EndTimer
  (Utilities|Time|ClearandInvalidateTimerbyHandle (Variables|Timers|GetTimerHandle))
  (CallFunction|PlaySeqArr (stale Custom|PlaySeqArr Sequences) (stale Custom|PlaySeqArr PauseAtSeq) (stale Custom|PlaySeqArr SeqToPause)))

(event Custom|OnPause_Event_0
  (CallFunction|CreateTimer 10))

(fn ConstructionScript)

(fn GetClashSequence
  (params (TeamTag :type Name))
  (if (Class|BPFunctionLibrary|IsTeam1 TeamTag)
    (return "/Game/Cinematics/Sequences/AnimationStateSequence/Characters_StateClash_02.Characters_StateClash_02")
    (else
      (return "/Game/Cinematics/Sequences/AnimationStateSequence/Characters_StateClash_01.Characters_StateClash_01"))))

(fn SetHUDReference
  (params (MenuHUD :type HUD%20Game%20Object%20Reference))
  (bind _output_get (Variables|Default|SetMenuHUD MenuHUD))
  (Utilities|IsValid _output_get
    (:Is%20Valid
      (Development|PrintString "Set reference to the hud successfuly"))
    (:Is%20Not%20Valid
      (Development|PrintString "Set reference to the hud unsuccessfuly")))
  (return))

(fn HidePlayMenu
  (bind _menuhud (Variables|Default|GetMenuHUD))
  (Utilities|IsValid _menuhud
    (:Is%20Valid
      (Default|HideMasterHUD _menuhud))
    (:Is%20Not%20Valid
      _))
  (return))

(fn ShowPlayMenu
  (bind _menuhud (Variables|Default|GetMenuHUD))
  (Utilities|IsValid _menuhud
    (:Is%20Valid
      (Default|ShowMasterHUD _menuhud))
    (:Is%20Not%20Valid
      _))
  (return))

(fn SetDefaultValuesClashSequence
  (Variables|Local|SetClashSeqOneIn (Variables|Defaultvalues|GetDefaultClashSequenceOne))
  (Variables|Local|SetSelectedSequenceTwoClash (Variables|Defaultvalues|GetDefaultClashSequenceTwoClash)))

(fn SetSeqChoiceClash2
  (params (SelectedSequenceTwoClash :type Level%20Sequence%20Object%20Reference))
  (Variables|Local|SetSelectedSequenceTwoClash SelectedSequenceTwoClash))