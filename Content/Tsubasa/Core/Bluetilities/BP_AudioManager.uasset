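; Audio manager that plays looping background music playlists for the home menu and the in-game field.
; Each track spawns as a 2D sound, and its finished event increments the index, wrapping at the end, then plays the next one.
; Both playlists share one track index and one current audio component.
; Volume initializes from game settings and can update the playing track, while NextTrack destroys the current component.
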(event Custom|PlayHomeTrackMusic
  ;[1 1 1] Main audio loop for the menu
  (bind _audiocomponent (CallFunction|PlayLoop (Variables|Default|GetCurrentTrackIndex) (Variables|Default|GetHomePlaylistLength) (Variables|Default|GetHomeBackgroundMusic)))
  (EventDispatchers|BindEventtoOnAudioFinished _audiocomponent (delegate Custom|HomeTrackLoop)))

(event Custom|HomeTrackLoop
  ;[1 1 1] Main audio loop for the menu
  (CallFunction|IncrementTrack (Variables|Default|GetHomePlaylistLength))
  (CallFunction|PlayHomeTrackMusic))

(event Custom|PlayFieldTrackMusic
  ;[1 1 1] Main audio loop for the in-game music
  (bind _audiocomponent (CallFunction|PlayLoop (Variables|Default|GetCurrentTrackIndex) (Variables|Default|GetFieldPlaylistLength) (Variables|Default|GetBackgroundFieldMuisc)))
  (EventDispatchers|BindEventtoOnAudioFinished _audiocomponent (delegate Custom|FieldTrackLoop)))

(event Custom|FieldTrackLoop
  ;[1 1 1] Main audio loop for the in-game music
  (CallFunction|IncrementTrack (Variables|Default|GetFieldPlaylistLength))
  (CallFunction|PlayFieldTrackMusic))

(event EventBeginPlay
  (Utilities|FlowControl|Sequence
    (:then_0
      (Variables|Default|SetHomePlaylistLength (Utilities|Array|Length (Variables|Default|GetHomeBackgroundMusic))))
    (:then_1
      (Variables|Default|SetFieldPlaylistLength (Utilities|Array|Length (Variables|Default|GetBackgroundFieldMuisc))))))

(fn ConstructionScript)

(fn StartBackgroundMusic
  (CallFunction|PlayHomeTrackMusic))

(fn StartFieldMusic
  (CallFunction|PlayFieldTrackMusic))

(fn PlayTrackfromPlaylist
  (params (PlaylistLength :type Integer) (Playlist :type Array%20of%20Sound%20Wave%20Object%20References) (TrackIndex :type Integer))
  (if (== PlaylistLength 0)
    (Development|PrintString "Empty playlist.")
    (else
      (bind _returnvalue (Audio|SpawnSound2D (Utilities|Array|Get(acopy) Playlist TrackIndex) (Variables|Default|GetAudioVolume) 1.0 0.0 0))
      (return _returnvalue))))

(fn SetVolume
  (params (NewVolume :type Float%20%28single-precision%29))
  (bind _output_get (Variables|Default|SetAudioVolume NewVolume))
  (Audio|Components|Audio|SetVolumeMultiplier (Variables|Default|GetCurrentTrackAudioComponent) _output_get :!class /Script/Engine.AudioComponent))

(fn NextTrack
  (Components|DestroyComponent (Variables|Default|GetCurrentTrackAudioComponent))
  (return))

(fn GetVolume
  (return (Variables|Default|GetAudioVolume)))

(fn PlayLoop
  (params (TrackIndex :type Integer) (PlaylistLength :type Integer) (Playlist :type Array%20of%20Sound%20Wave%20Object%20References))
  (bind _audiocomponent (CallFunction|PlayTrackfromPlaylist PlaylistLength Playlist TrackIndex))
  (Variables|Default|SetCurrentTrackAudioComponent _audiocomponent)
  (return _audiocomponent))

(fn IncrementTrack
  (params (PlaylistLength :type Integer))
  (if (== PlaylistLength 0)
    (Development|PrintString "EmptyPlaylist" false true "(R=1.000000,G=0.164236,B=0.000000,A=1.000000)")
    (else
      (Variables|Default|SetCurrentTrackIndex (+ (Variables|Default|GetCurrentTrackIndex) 1))
      (if (not (> (Variables|Default|GetCurrentTrackIndex) (- PlaylistLength 1)))
        _
        (else
          (Variables|Default|SetCurrentTrackIndex 0)))))
  (Development|PrintString (Utilities|String|Append "Next track: " (Utilities|String|ToString(Integer) (Variables|Default|GetCurrentTrackIndex))) false)
  (return))

(fn Init
  (params (GameSettings :type Game%20Settings%20Structure))
  (Utilities|FlowControl|Sequence
    (:then_0
      (Variables|Default|SetAudioVolume (Utilities|Struct|BreakGameSettings GameSettings)))))