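; Sequence manager that plays clash and player-ability cinematics and hides the master HUD while they run.
; Clash IDs pick sequences from a clash DataTable, after the tagged enemy puppet is recolored through a dynamic material.
; Ability names resolve through attacker, guard or goalie tables by player role.
; ClashAbility hides puppet meshes and chains clash into ability via OnFinished, whose final callback restores the HUD.
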(event Custom|PlaySequenceDebug
  (params (AbilityName :type Name))
  (bind _returnvalue (CallFunction|PlaySequencefromList AbilityName))
  (CallFunction|FinishedBindEvent _returnvalue))

(event Custom|FinishedSequenceEvent
  (Development|PrintString "Finished with the sequence")
  (bind _hud (Variables|Default|GetHUD)
    (:then
      (Default|ShowMasterHUD _hud))
    (:else
      (Development|PrintString "Not valid hud reference"))))

(event Custom|FinishedBindEvent
  (params (LevelSequence :type Level%20Sequence%20Player%20Object%20Reference%20%28by%20ref%29))
  (EventDispatchers|BindEventtoOnFinished LevelSequence (delegate Custom|FinishedSequenceEvent)))

(event Custom|PlayClashSequence
  (params (ID :type Integer))
  (bind _levelsequence (Utilities|ClashSequenceMacro ID "EnemyClash" "(R=0.147909,G=0.329976,B=1.000000,A=1.000000)"))
  (CallFunction|FinishedBindEvent _levelsequence))

(event Custom|PlaySequenceFromNameEvent
  (params (AbilityName :type Name) (PlayerRole :type EPlayerRole%20Enum :default "forward"))
  (bind _levelsequence (CallFunction|PlaySequencefromAbilityName AbilityName PlayerRole))
  (Utilities|IsValid _levelsequence
    (:Is%20Valid
      (CallFunction|FinishedBindEvent _levelsequence))))

(event Custom|ClashAbility
  (params (ClashID :type Integer) (AbilityName :type Name) (PlayerRole :type EPlayerRole%20Enum :default "forward"))
  (bind _outactors (Actor|GetAllActorsOfClass "/Game/Animations/RigsAndShit/BP_Puppet.BP_Puppet_C"))
  (for _array_element _outactors
    (Rendering|SetVisibility (Variables|/Game/Animations/RigsAndShit/BP_Puppet.BP_Puppet_C|GetSkeletalMesh _array_element) false true))
  (bind _levelsequence (Utilities|ClashSequenceMacro ClashID "EnemyClash" (Variables|Default|GetEnemyColorUniform)))
  (EventDispatchers|BindEventtoOnFinished _levelsequence (delegate Custom|AbilitySeq))
  (Variables|Default|SetCurrentAbilityName AbilityName)
  (Variables|Default|SetCurrentRole PlayerRole))

(event Custom|AbilitySeq
  (bind _levelsequence (CallFunction|PlaySequencefromAbilityName (Variables|Default|GetCurrentAbilityName) (Variables|Default|GetCurrentRole)))
  (CallFunction|FinishedBindEvent _levelsequence))

(event EventBeginPlay)

(fn ConstructionScript)

(fn PlaySequencefromList
  (params (AbilityName :type Name%20%28by%20ref%29))
  (bind _hud (Variables|Default|GetHUD)
    (:then
      (Default|HideMasterHUD _hud))
    (:else
      (Development|PrintString "Not valid hide")))
  (bind _returnvalue (Utilities|GetDataTableRow "/Game/Tsubasa/Core/Blueprints/Tables/Sequences/DT_AttackerSequences.DT_AttackerSequences" "Backflip")
    (:then
      (bind _returnvalue_2 (Sequencer|Player|CreateLevelSequencePlayer (.Sequence (Utilities|Struct|BreakFSequnceDT _returnvalue)) (Utilities|Struct|MakeMovieSceneSequencePlaybackSettings false "(Value=0)" 1.0 0.0 false false false false false true)))
      (Sequencer|Player|Play _returnvalue_2 :!class /Script/MovieScene.MovieSceneSequencePlayer)
      (return _returnvalue_2))))

(fn PlaySequencefromAbilityName
  (params (AbilityName :type Name) (PlayerRole :type EPlayerRole%20Enum :default "forward"))
  (Utilities|FlowControl|Sequence
    (:then_0
      (switch Utilities|FlowControl|Switch|SwitchonEPlayerRole PlayerRole
        (:forward
          (bind _returnvalue (Utilities|GetDataTableRow "/Game/Tsubasa/Core/Blueprints/Tables/Sequences/DT_AttackerSequences.DT_AttackerSequences" AbilityName)
            (:then
              (bind _levelsequence (CallFunction|PlaySequenceInstance (.Sequence (Utilities|Struct|BreakFSequnceDT _returnvalue))))
              (return _levelsequence))))
        (:midfield
          (bind _returnvalue_2 (Utilities|GetDataTableRow "/Game/Tsubasa/Core/Blueprints/Tables/Sequences/DT_AttackerSequences.DT_AttackerSequences" AbilityName)
            (:then
              (bind _levelsequence_2 (CallFunction|PlaySequenceInstance (.Sequence (Utilities|Struct|BreakFSequnceDT _returnvalue_2))))
              (return _levelsequence_2))))
        (:defender
          (bind _returnvalue_3 (Utilities|GetDataTableRow "/Game/Tsubasa/Core/Blueprints/Tables/Sequences/DT_GuardSequences.DT_GuardSequences" AbilityName)
            (:then
              (bind _levelsequence_3 (CallFunction|PlaySequenceInstance (.Sequence (Utilities|Struct|BreakFSequnceDT _returnvalue_3))))
              (return _levelsequence_3))))
        (:goalkeeper
          (bind _returnvalue_4 (Utilities|GetDataTableRow "/Game/Tsubasa/Core/Blueprints/Tables/Sequences/DT_Goalie.DT_Goalie" AbilityName)
            (:then
              (bind _levelsequence_4 (CallFunction|PlaySequenceInstance (.Sequence (Utilities|Struct|BreakFSequnceDT _returnvalue_4))))
              (return _levelsequence_4))))))
    (:then_1
      (bind _hud (Variables|Default|GetHUD)
        (:then
          (Default|HideMasterHUD _hud))
        (:else)))))

(fn PlaySequenceInstance
  (params (NewParam :type Level%20Sequence%20Object%20Reference%20%28by%20ref%29))
  (bind _returnvalue (Sequencer|Player|CreateLevelSequencePlayer NewParam (Utilities|Struct|MakeMovieSceneSequencePlaybackSettings true "(Value=0)")))
  (Sequencer|Player|Play _returnvalue :!class /Script/MovieScene.MovieSceneSequencePlayer)
  (return _returnvalue))