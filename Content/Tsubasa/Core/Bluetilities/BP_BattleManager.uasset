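; Battle manager for football matches, coordinating both NPC teams, ball possession, player freezing and clash puppet looks.
; Spawn functions build both elevens from formation DataTables and player 1's inventory, which also supplies Team 2's players.
; A looping timer auto-passes the ball and restarts on pawn-to-pawn passes.
; Shots resolve by range and attack-versus-goalie stats, while score updates reset positions and hand the other team kickoff.
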(event Custom|PassBallTimer
  (bind _asfootball_character (Utilities|Casting|CastToFootballCharacter (Variables|Default|GetActorPossessingBall)))
  (Class|BattleManager|PassBalltoClosestTeammate _asfootball_character true 1e+04)
  (Development|PrintString "Passed ball by timer."))

(event Custom|ResetPassBallTimer
  (bind _returnvalue (Utilities|Time|SetTimerbyEvent (delegate Custom|PassBallTimer) (Variables|Default|GetPassBallCheckTime) true))
  (Variables|Default|SetPassBallTimerHandle _returnvalue))

(event EventBeginPlay
  (Utilities|FlowControl|Sequence
    (:then_0
      (Utilities|GrabBothTeamNPCs))
    (:then_1
      ;[1 1 1] Acquire the inventory of player 1
      (bind _aspc_stadium_game (Utilities|Casting|CastToPC_Stadium_Game (Game|GetPlayerController 0)))
      (Variables|Default|SetPlayerInventoryTeam1 (Variables|/Game/Tsubasa/Core/Blueprints/PlayerControllers/PC_Stadium_Game.PC_Stadium_Game_C|GetPlayerInventory _aspc_stadium_game)))
    (:then_2
      ;[1 1 1] Get actor possessing ball [debug]
      (bind _actorpossessingball (CallFunction|GetActorPossessingBall))
      (Variables|Default|SetActorPossessingBall _actorpossessingball)
      (Utilities|Time|SetTimerbyFunctionName 0 "DetermineStates" 2.0 true))
    (:then_3
      (CallFunction|BindEvt)
      (bind _returnvalue (Utilities|Time|SetTimerbyEvent (delegate Custom|PassBallTimer) (Variables|Default|GetPassBallCheckTime) true))
      (Variables|Default|SetPassBallTimerHandle _returnvalue))))

(event Custom|T1HasBallEvent
  (Class|BattleManager|CallT1HasBall))

(event Custom|BallIsInGoalEvent
  (Class|BattleManager|CallBallIsinGoalStates))

(event Custom|T2HasBallEvent
  (Class|BattleManager|CallT2HasBall))

(event Custom|BindEvt
  (EventDispatchers|AssignOnScoreUpdate (Subsystems|GetScoreSubsystem) (delegate Custom|OnScoreUpdate_Event_0)))

(event Custom|OnScoreUpdate_Event_0
  (params (TeamID :type Integer))
  (CallFunction|ScoreGoalHandler TeamID)
  (Development|PrintString "Score goal handler triggered." true true "(R=0.040753,G=1.000000,B=0.000000,A=1.000000)"))

(event Custom|FreezePlayers
  (Default|CallStopAllInactivePWN))

(event Custom|UnfreezePlayers
  (Default|CallStartAllInactivePWN)
  (Default|CallResetPWNPlayerTurn))

(event Custom|FreezePlayersExcept
  (params (PWNException :type PWN%20NPC%20Object%20Reference%20%28by%20ref%29))
  (Variables|/Game/Tsubasa/Core/Blueprints/Characters/PWN_NPC.PWN_NPC_C|SetbPlayerTurn PWNException true)
  (CallFunction|FreezePlayers))

(event EventCallBallIsinGoalStates
  (|CallParentFunction)
  (for _index (range 0 (- (Utilities|Array|Length (Variables|Default|GetTeam1PWN_NPC)) 1))
    (Utilities|IsValid (Utilities|Array|Get(acopy) (Variables|Default|GetTeam1PWN_NPC) _index)
      (:Is%20Valid
        (Class|FootballCharacter|BallIsinGoalState (Utilities|Array|Get(acopy) (Variables|Default|GetTeam1PWN_NPC) _index))
        (Utilities|IsValid (Utilities|Array|Get(acopy) (Variables|Default|GetTeam2PWN_NPC) _index)
          (:Is%20Valid
            (Class|FootballCharacter|BallIsinGoalState (Utilities|Array|Get(acopy) (Variables|Default|GetTeam2PWN_NPC) _index))))))))

(fn ConstructionScript)

(fn PassBalltoEnemyIntercepted)

(fn SpawnTeam2
  (bind _playerinventoryteam1 (Variables|Default|GetPlayerInventoryTeam1))
  (bind (_activeplayers _activereserveplayers _allplayers _profilestruct _playerformation) (Utilities|Struct|BreakFPlayerInventory _playerinventoryteam1))
  (Utilities|FlowControl|Sequence
    (:then_0
      (switch Utilities|FlowControl|Switch|SwitchonEPlayerPositions _playerformation
        (:NewEnumerator0
          _)
        (:NewEnumerator1
          _))
      (bind _returnvalue (Utilities|GetDataTableRow "/Game/Tsubasa/Core/Blueprints/Tables/PlayerLayouts/DT_EnemyLayoutPositions.DT_EnemyLayoutPositions" "EP_343")
        (:then
          (LocalVariables|SetFoundRow _returnvalue))))
    (:then_2
      (for _index (range 0 10)
        (bind _returnvalue_2 (Game|SpawnActorfromClass "/Game/Tsubasa/Core/Blueprints/Characters/PWN_NPC.PWN_NPC_C" (Math|Transform|MakeTransform (Math|Vector|MakeVector (.x (Utilities|Array|Get(acopy) (.Location (Utilities|Struct|BreakFLayoutPosition (LocalVariables|GetFoundRow))) _index)) (.y (Utilities|Array|Get(acopy) (.Location (Utilities|Struct|BreakFLayoutPosition (LocalVariables|GetFoundRow))) _index)) (+ (.z (Utilities|Array|Get(acopy) (.Location (Utilities|Struct|BreakFLayoutPosition (LocalVariables|GetFoundRow))) _index)) 1e+02)) "0, 0, 0" (.Scale (Utilities|Struct|BreakFLayoutPosition (LocalVariables|GetFoundRow)))) "Undefined" 0 0))
        (Default|InitiatePawn _returnvalue_2 self (Variables|Default|GetGoalGateT2Ref) (Utilities|Array|Get(acopy) _activeplayers _index) (Variables|Default|GetTagArrayTeam2) true)
        (Utilities|Array|Add (Variables|Default|GetTeam2PWN_NPC) _returnvalue_2)
        (Utilities|Array|Add (Variables|Default|GetT2PWNArray) _returnvalue_2)
        (Development|PrintString (Utilities|String|Append "spawned: " (Utilities|GetDisplayName _returnvalue_2)) false true "(R=0.162855,G=1.000000,B=0.000000,A=1.000000)")
        (if (Utilities|Enum|Equal(Enum) (.PlayerRole (Utilities|Struct|BreakPlayerProperties (Utilities|Array|Get(acopy) _activeplayers _index))) "goalkeeper")
          (Default|SetGoalStats (Variables|Default|GetGoalGateT2Ref) (.CoreStats (Utilities|Struct|BreakPlayerProperties (Utilities|Array|Get(acopy) _activeplayers _index))))))
      (bind _asaic_npc (Utilities|Casting|CastToAIC_NPC (AI|GetAIController _returnvalue_2)))
      (Default|RunNPCBT _asaic_npc))))

(fn SpawnTeam1
  (params (StartingBallTeam :type Boolean))
  (Utilities|FlowControl|Sequence
    (:then_0
      (switch Utilities|FlowControl|Switch|SwitchonEPlayerPositions (Utilities|Struct|BreakFPlayerInventory (Variables|Default|GetPlayerInventoryTeam1))
        (:NewEnumerator0
          (bind _returnvalue (Utilities|GetDataTableRow "/Game/Tsubasa/Core/Blueprints/Tables/PlayerLayouts/DT_LayoutPositions.DT_LayoutPositions" "EP_343")
            (:then
              (LocalVariables|SetFoundRow _returnvalue))))
        (:NewEnumerator1
          (bind _returnvalue_2 (Utilities|GetDataTableRow "/Game/Tsubasa/Core/Blueprints/Tables/PlayerLayouts/DT_LayoutPositions.DT_LayoutPositions" "EP_242")
            (:then
              (LocalVariables|SetFoundRow _returnvalue_2))))))
    (:then_1
      (for _index (range 0 10)
        (bind _output_get (LocalVariables|SetIndex _index))
        (bind _returnvalue_3 (Game|SpawnActorfromClass "/Game/Tsubasa/Core/Blueprints/Characters/PWN_NPC.PWN_NPC_C" (Math|Transform|MakeTransform (Math|Vector|MakeVector (.x (Utilities|Array|Get(acopy) (.Location (Utilities|Struct|BreakFLayoutPosition (LocalVariables|GetFoundRow))) _output_get)) (.y (Utilities|Array|Get(acopy) (.Location (Utilities|Struct|BreakFLayoutPosition (LocalVariables|GetFoundRow))) _output_get)) (+ (.z (Utilities|Array|Get(acopy) (.Location (Utilities|Struct|BreakFLayoutPosition (LocalVariables|GetFoundRow))) _output_get)) 1e+02)) "0, 0, 0" (.Scale (Utilities|Struct|BreakFLayoutPosition (LocalVariables|GetFoundRow)))) "AdjustIfPossibleButAlwaysSpawn" 0 0))
        (LocalVariables|SetCurrentPWN _returnvalue_3)
        (Utilities|FlowControl|Sequence
          (:then_0
            (Default|InitiatePawn (LocalVariables|GetCurrentPWN) self (Variables|Default|GetGoalGateT1Ref) (Utilities|Array|Get(acopy) (Utilities|Struct|BreakFPlayerInventory (Variables|Default|GetPlayerInventoryTeam1)) (LocalVariables|GetIndex)) (Variables|Default|GetTagArrayTeam1) true))
          (:then_1
            (Utilities|Array|Add (Variables|Default|GetTeam1PWN_NPC) (LocalVariables|GetCurrentPWN))
            (Utilities|Array|Add (Variables|Default|GetT1PWNArray) (LocalVariables|GetCurrentPWN)))
          (:then_2
            (if (Utilities|Enum|Equal(Enum) (.PlayerRole (Utilities|Struct|BreakPlayerProperties (Utilities|Array|Get(acopy) (Utilities|Struct|BreakFPlayerInventory (Variables|Default|GetPlayerInventoryTeam1)) (LocalVariables|GetIndex)))) "goalkeeper")
              (Default|SetGoalStats (Variables|Default|GetGoalGateT1Ref) (.CoreStats (Utilities|Struct|BreakPlayerProperties (Utilities|Array|Get(acopy) (Utilities|Struct|BreakFPlayerInventory (Variables|Default|GetPlayerInventoryTeam1)) (LocalVariables|GetIndex)))))
              (Variables|Default|SetGoalieT1 (LocalVariables|GetCurrentPWN))))
          (:then_3
            (if (and (== (LocalVariables|GetIndex) 9) StartingBallTeam)
              (Class|BattleManager|SetupStartingPawnwithBall (LocalVariables|GetCurrentPWN)))))))))

(fn SpawnTeam2Bots
  (params (StartingBallTeam :type Boolean))
  (bind _playerinventoryteam1 (Variables|Default|GetPlayerInventoryTeam1))
  (bind (_activeplayers _activereserveplayers _allplayers _profilestruct _playerformation) (Utilities|Struct|BreakFPlayerInventory _playerinventoryteam1))
  (Utilities|FlowControl|Sequence
    (:then_0
      (switch Utilities|FlowControl|Switch|SwitchonEPlayerPositions _playerformation
        (:NewEnumerator0
          _)
        (:NewEnumerator1
          _))
      (bind _returnvalue (Utilities|GetDataTableRow "/Game/Tsubasa/Core/Blueprints/Tables/PlayerLayouts/DT_EnemyLayoutPositions.DT_EnemyLayoutPositions" "EP_343")
        (:then
          (LocalVariables|SetFoundRow _returnvalue))))
    (:then_2
      (for _index (range 0 10)
        (bind _output_get (LocalVariables|SetIndex _index))
        (bind _returnvalue_2 (Game|SpawnActorfromClass "/Game/Tsubasa/Core/Blueprints/Characters/PWN_NPC.PWN_NPC_C" (Math|Transform|MakeTransform (Math|Vector|MakeVector (.x (Utilities|Array|Get(acopy) (.Location (Utilities|Struct|BreakFLayoutPosition (LocalVariables|GetFoundRow))) _output_get)) (.y (Utilities|Array|Get(acopy) (.Location (Utilities|Struct|BreakFLayoutPosition (LocalVariables|GetFoundRow))) _output_get)) (+ (.z (Utilities|Array|Get(acopy) (.Location (Utilities|Struct|BreakFLayoutPosition (LocalVariables|GetFoundRow))) _output_get)) 1e+02)) "0, 0, 0" (.Scale (Utilities|Struct|BreakFLayoutPosition (LocalVariables|GetFoundRow)))) "Undefined" 0 0))
        (bind _output_get_2 (LocalVariables|SetPWN _returnvalue_2))
        (Default|InitiatePawn _output_get_2 self (Variables|Default|GetGoalGateT2Ref) (Utilities|Array|Get(acopy) _activeplayers (LocalVariables|GetIndex)) (Variables|Default|GetTagArrayTeam2) true)
        (Utilities|Array|Add (Variables|Default|GetTeam2PWN_NPC) (LocalVariables|GetPWN))
        (Utilities|Array|Add (Variables|Default|GetT2PWNArray) (LocalVariables|GetPWN))
        (Utilities|FlowControl|Sequence
          (:then_0
            ;[1 1 1] set the goalie reference
            (if (Utilities|Enum|Equal(Enum) (.PlayerRole (Utilities|Struct|BreakPlayerProperties (Utilities|Array|Get(acopy) _activeplayers (LocalVariables|GetIndex)))) "goalkeeper")
              (Default|SetGoalStats (Variables|Default|GetGoalGateT2Ref) (.CoreStats (Utilities|Struct|BreakPlayerProperties (Utilities|Array|Get(acopy) _activeplayers (LocalVariables|GetIndex)))))
              (Variables|Default|SetGoalieT2 (LocalVariables|GetPWN))))
          (:then_1
            ;[1 1 1] set as starting pawn
            (if (and (== (LocalVariables|GetIndex) 9) StartingBallTeam)
              (Class|BattleManager|SetupStartingPawnwithBall (LocalVariables|GetPWN)))))))))

(fn SetupReferences
  (Utilities|FlowControl|Sequence
    (:then_0
      (bind _outactors (Actor|GetAllActorsOfClasswithTag "/Game/Tsubasa/Core/Blueprints/Actors/ACT_Goal.ACT_Goal_C" "TargetGateForT1"))
      (bind _asact_goal (Utilities|Casting|CastToACT_Goal (Utilities|Array|Get(acopy) _outactors)))
      (Variables|Default|SetGoalGateT1Ref _asact_goal))
    (:then_1
      (bind _outactors_2 (Actor|GetAllActorsOfClasswithTag "/Game/Tsubasa/Core/Blueprints/Actors/ACT_Goal.ACT_Goal_C" "TargetGateForT2"))
      (bind _asact_goal_2 (Utilities|Casting|CastToACT_Goal (Utilities|Array|Get(acopy) _outactors_2)))
      (Variables|Default|SetGoalGateT2Ref _asact_goal_2))))

(fn ChangeBallPossessorClashPuppetMaterials
  (params (Player%20Props :type Player%20Properties%20Structure) (IsClash01 :type Boolean))
  (bind (_playerrole _hairmeshid _haircolor _skincolor _skinshade _clothescolor) (Utilities|Struct|BreakPlayerProperties Player%20Props))
  (if IsClash01
    (LocalVariables|SetClashName (LocalVariables|GetClashName01))
    (else
      (LocalVariables|SetClashName (LocalVariables|GetClashName02))))
  (bind _outactors (Actor|GetAllActorswithTag (LocalVariables|GetClashName)))
  (bind _asbp_puppet (Utilities|Casting|CastToBP_Puppet (Utilities|Array|Get(acopy) _outactors)))
  (Default|SetupPuppet _asbp_puppet _hairmeshid _haircolor _clothescolor _skincolor _playerrole 0.4))

(fn ScoreGoalMatchup
  (params (Attacker :type PWN%20NPC%20Object%20Reference%20%28by%20ref%29) (KickRange :type Integer))
  (bind _returnvalue (Transformation|GetActorLocation Attacker))
  (bind _returnvalue_2 (Math|Conversions|ToFloat(Integer) KickRange))
  (bind _goalreference (Variables|/Script/AIProject.FootballCharacter|GetGoalReference Attacker))
  (bind _returnvalue_3 (Transformation|GetActorLocation _goalreference))
  (bind _returnvalue_4 (Math|Vector|Distance(Vector) _returnvalue _returnvalue_3))
  (bind _returnvalue_5 (<= _returnvalue_4 _returnvalue_2))
  (Utilities|FlowControl|Sequence
    (:then_0
      (Development|PrintString (Utilities|String|Append (Utilities|String|ToString(Boolean) (Utilities|IsValid (Variables|Default|GetGoalieT1))) " " (Utilities|String|ToString(Boolean) (Utilities|IsValid (Variables|Default|GetGoalieT2))))))
    (:then_1
      (Utilities|IsValid Attacker
        (:Is%20Valid
          (if (Class|FootballCharacter|IsTeam1 Attacker)
            (LocalVariables|SetTargetGoalie (Variables|Default|GetGoalieT1))
            (else
              (LocalVariables|SetTargetGoalie (Variables|Default|GetGoalieT2))))
          (Development|PrintString (Utilities|String|Append "In range for goal: " (Utilities|String|ToString(Boolean) _returnvalue_5)) true false)
          (if (and (Class|BattleManager|GetOutcomeAttack (Utilities|Struct|BreakPlayerCoreStats (.CoreStats (Utilities|Struct|BreakPlayerProperties (Variables|/Script/AIProject.FootballCharacter|GetPlayerProperties Attacker)))) (Utilities|Struct|BreakPlayerCoreStats (.CoreStats (Utilities|Struct|BreakPlayerProperties (Variables|/Script/AIProject.FootballCharacter|GetPlayerProperties (LocalVariables|GetTargetGoalie))))) true 1.0 3e+02) _returnvalue_5)
            (Default|KickBallinGoal Attacker false)
            (return true)
            (elif _returnvalue_5
              (Class|FootballCharacter|EnemyGoalieHasBall Attacker)
              (if (Class|FootballCharacter|IsTeam1 Attacker)
                (Default|CallT1HasBall false)
                (bind _goaliet2 (Variables|Default|GetGoalieT2)
                  (:then
                    (Class|FootballCharacter|ReceiveBall _goaliet2))
                  (:else
                    _))
                (else
                  (Default|CallT1HasBall true)
                  (bind _goaliet1 (Variables|Default|GetGoalieT1)
                    (:then
                      (Class|FootballCharacter|ReceiveBall _goaliet1))
                    (:else
                      _))))
              (return false)
              (else
                (return false)))))
        (:Is%20Not%20Valid
          (Development|PrintString "GoalMatchup Invalid attacker."))))))

(fn ScoreGoalHandler
  (params (TeamID :type Integer))
  (bind _returnvalue (Class|KismetSystemLibrary|MakeLiteralInteger 9))
  (bind _team1pwn_npc (Variables|Default|GetTeam1PWN_NPC))
  (bind _team2pwn_npc (Variables|Default|GetTeam2PWN_NPC))
  (Default|CallResetPlayerLocations)
  (switch int TeamID
    (:1
      (if (Utilities|Array|IsValidIndex _team2pwn_npc _returnvalue)
        (Class|BattleManager|SetupStartingPawnwithBall (Utilities|Array|Get(acopy) _team2pwn_npc _returnvalue))
        (return)
        (else
          _)))
    (:2
      (if (Utilities|Array|IsValidIndex _team1pwn_npc _returnvalue)
        (Class|BattleManager|SetupStartingPawnwithBall (Utilities|Array|Get(acopy) _team1pwn_npc _returnvalue))
        (return)
        (else
          _))))
  (Development|PrintString "Other teamd doesn't exist to hand over the ball, ScoreGoalHandle" false))

(fn PassBallfromPwntoPwn
  (params (Initiator :type Football%20Character%20Object%20Reference) (IdealPassMate :type Football%20Character%20Object%20Reference))
  (bind _returnvalue (|CallParentFunction Initiator IdealPassMate))
  (Default|CallBallPassedPWNtoPWN)
  (CallFunction|ResetPassBallTimer)
  (return _returnvalue))

(fn ChangeFriendlyPuppetMaterials
  (params (Tag :type Name) (Player%20Props :type Player%20Properties%20Structure))
  (bind (_playerrole _hairmeshid _haircolor _skincolor _skinshade _clothescolor) (Utilities|Struct|BreakPlayerProperties Player%20Props))
  (bind _outactors (Actor|GetAllActorswithTag Tag))
  (bind _asbp_puppet (Utilities|Casting|CastToBP_Puppet (Utilities|Array|Get(acopy) _outactors)))
  (Default|SetupPuppet _asbp_puppet _hairmeshid _haircolor _clothescolor _skincolor _playerrole 0.4))

(fn SetupHandOffValues
  (params (PWNAttacking :type Football%20Character%20Object%20Reference) (PWNBeingAttacked :type Football%20Character%20Object%20Reference))
  (Variables|Default|SetPWNAttacking PWNAttacking)
  (Variables|Default|SetPWNBeingAttacked PWNBeingAttacked)
  (return))