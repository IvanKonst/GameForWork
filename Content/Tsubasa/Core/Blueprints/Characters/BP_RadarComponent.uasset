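; BP_RadarComponent is a component that registers its owning actor with the radar on the game HUD.
; The AddToRadar event casts the first player controller's HUD to HUD_Game, adds the owner as a radar actor and prints a debug string.
; EndPlay removes the owner through the same HUD lookup, while registration relies on AddToRadar being called, as the component has no BeginPlay logic.
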(event Custom|AddToRadar
  (bind _returnvalue (Game|GetPlayerController 0))
  (Utilities|IsValid _returnvalue
    (:Is%20Valid
      (bind _ashud_game (Utilities|Casting|CastToHUD_Game (HUD|GetHUD _returnvalue)))
      (Default|AddRadarActor _ashud_game (Components|GetOwner))
      (Development|PrintString "Added to radar"))))

(event EventEndPlay
  (params (EndPlayReason :type EEndPlayReason%20Enum :default "Destroyed"))
  (bind _returnvalue (Game|GetPlayerController 0))
  (Utilities|IsValid _returnvalue
    (:Is%20Valid
      (bind _ashud_game (Utilities|Casting|CastToHUD_Game (HUD|GetHUD _returnvalue)))
      (Default|RemoveRadarActor _ashud_game (Components|GetOwner)))))