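; AI-driven football character pawn that switches between NPC and player-turn behavior trees on its AIC_NPC controller.
; BattleManager delegates stop, restart or teleport it and set team possession states, which a timer and state-change delegate copy to the blackboard.
; Triggered abilities spend stamina, then either start a SequenceManager clash or the player-turn tree.
; It also wraps parent ball events to refresh the possession widget and runs a timer-based skill cooldown.
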(event Custom|UpdateBlackboardState
  (bind _aicontrollerreference (Variables|Default|GetAIControllerReference)
    (:then
      (bind _blackboard (Variables|/Script/AIModule.AIController|GetBlackboard _aicontrollerreference)
        (:then
          (CallFunction|UpdateBlackboardStates _blackboard))
        (:else)))
    (:else
      (Development|PrintString "AIController reference is invalid"))))

(event EventBeginPlay
  (Utilities|FlowControl|Sequence
    (:then_0
      ;[1 1 1] Launch the BT
      (bind _asaic_npc (Utilities|Casting|CastToAIC_NPC (AI|GetAIController self)))
      (bind _output_get (Variables|Default|SetAIControllerReference _asaic_npc))
      (Default|RunNPCBT _output_get))
    (:then_1
      ;[1 1 1] Grab reference of BP_Battlemanager
      (bind _returnvalue (Actor|GetActorOfClass "/Game/Tsubasa/Core/Bluetilities/BP_BattleManager.BP_BattleManager_C"))
      (Variables|Default|SetBattleManager _returnvalue))
    (:then_2
      (CallFunction|BindEvent))
    (:then_3
      (Utilities|FlowControl|Delay 0.2)
      (Utilities|Time|SetTimerbyEvent (delegate Custom|UpdateBlackboardState) 0.5 true)
      (EventDispatchers|BindEventtoChangedStateDelegate (delegate Custom|UpdateBlackboardState)))))

(event Custom|CallEnemyHasBall
  (Class|FootballCharacter|EnemyHasBall)
  (Default|CallUpdateHasBallPWidget))

(event Custom|CallBallIsInGoal
  (Class|FootballCharacter|BallIsinGoalState)
  (Default|CallUpdateHasBallPWidget))

(event Custom|CallTeammateHasBall
  (Class|FootballCharacter|TeammateHasBall)
  (Default|CallUpdateHasBallPWidget))

(event EventKickBallinGoal
  (params (CheckIfGoalIsValid :type Boolean))
  (|CallParentFunction CheckIfGoalIsValid)
  (Default|CallUpdateHasBallPWidget))

(event EventPassBall
  (params (IsInitiatingPass :type Boolean) (IsSuccessful :type Boolean))
  (|CallParentFunction IsInitiatingPass IsSuccessful)
  (Default|CallUpdateHasBallPWidget))

(event EventLoseBall
  (|CallParentFunction)
  (Default|CallUpdateHasBallPWidget))

(event EventSetVisibilityBall
  (params (Visible :type Boolean))
  (Rendering|SetVisibility (Variables|Default|GetSphere) Visible false)
  (if Visible
    (Default|CallUpdateHasBallPWidget)))

(event EventBall
  (|CallParentFunction)
  (Default|CallUpdateHasBallPWidget))

(event Custom|ActivateCooldownTimer
  (bind _returnvalue (Utilities|Time|SetTimerbyEvent (delegate Custom|ResetCooldown) (Variables|Default|GetSkillCooldown)))
  (Variables|Default|SetCooldownTimer _returnvalue))

(event Custom|ResetCooldown
  (Variables|Default|SetIsInCooldown false)
  (Utilities|Time|ClearandInvalidateTimerbyHandle (Variables|Default|GetCooldownTimer)))

(event Custom|ResetCooldownTimer
  (if (Utilities|Time|IsTimerActivebyHandle (Variables|Default|GetCooldownTimer))
    (Utilities|Time|ClearandInvalidateTimerbyHandle (Variables|Default|GetCooldownTimer)))
  (CallFunction|ActivateCooldown "Reset cooldown timer"))

(event Custom|StartAllPWN_Event_0
  (CallFunction|StartBT))

(event Custom|StopAllPWN_Event_0
  (CallFunction|StopBTifInactive))

(event Custom|ResetPWNPlayerTurn_Event_0
  (Variables|Default|SetbPlayerTurn false))

(event Custom|T1HasBall_Event_0
  (params (T1_Has_Ball :type Boolean))
  (bind _self self)
  (bind _returnvalue (Class|FootballCharacter|IsTeam1 _self))
  (if T1_Has_Ball
    (if _returnvalue
      (Class|FootballCharacter|TeammateHasBall)
      (else
        (Class|FootballCharacter|EnemyHasBall)))
    (elif _returnvalue
      (Class|FootballCharacter|EnemyHasBall)
      (else
        (Class|FootballCharacter|TeammateHasBall)))))

(event Custom|BindEvent
  (bind _battlemanager (Variables|Default|GetBattleManager))
  (Utilities|FlowControl|Sequence
    (:then_0
      (EventDispatchers|AssignStartAllInactivePWN _battlemanager (delegate Custom|StartAllPWN_Event_0))
      (EventDispatchers|AssignStopAllInactivePWN _battlemanager (delegate Custom|StopAllPWN_Event_0))
      (EventDispatchers|AssignResetPWNPlayerTurn _battlemanager (delegate Custom|ResetPWNPlayerTurn_Event_0))
      (EventDispatchers|AssignT1HasBall _battlemanager (delegate Custom|T1HasBall_Event_0))
      ;[1 1 1] Stop the player on end game event ( timer's out )
      (EventDispatchers|BindEventtoStopBTDelegate (Variables|Default|GetBattleManager) (delegate Custom|StopEndGameEvent)))
    (:then_1
      (EventDispatchers|AssignResetPlayerLocations (Variables|Default|GetBattleManager) (delegate Custom|ResetPlayerLocations_Event_0)))))

(event Custom|ResetPlayerLocations_Event_0
  (CallFunction|TeleporttoStartLocation))

(event Custom|StopEndGameEvent
  ;[1 1 1] Stop the player on end game event ( timer's out )
  (Default|StopBT (Variables|Default|GetAIControllerReference)))

(fn ConstructionScript)

(fn InitiatePawn
  (params (BP_BattleManagerReference :type BP%20Battle%20Manager%20Object%20Reference) (GoalReference :type Goal%20Gate%20Object%20Reference%20%28by%20ref%29) (PlayerProperties :type Player%20Properties%20Structure%20%28by%20ref%29) (TagsIn :type Array%20of%20Names) (SetDefaultAbilities :type Boolean))
  (Utilities|FlowControl|Sequence
    (:then_0
      (bind _output_get (Variables|Default|SetBattleManager BP_BattleManagerReference))
      (Variables|Default|SetBattleManagerReference _output_get))
    (:then_1
      (Variables|Default|SetGoalReference GoalReference))
    (:then_2
      (Variables|Default|SetPlayerProperties PlayerProperties))
    (:then_3
      (Variables|Default|SetTags TagsIn))
    (:then_4
      (Class|FootballCharacter|CalculateFieldPositions))
    (:then_5
      (if SetDefaultAbilities
        (Class|FootballCharacter|DefaultAbilityFactory)))))

(fn SeekEnemy
  (params (DistanceNearThreshold_In :type Float%20%28single-precision%29))
  (bind _returnvalue (Class|FootballCharacter|IsTeam1))
  (bind _battlemanager (Variables|Default|GetBattleManager))
  (bind _battlemanager_2 (Variables|Default|GetBattleManager))
  (bind _actorpossessingball (Variables|/Script/AIProject.BattleManager|GetActorPossessingBall _battlemanager))
  (bind _team2pwn_npc (Variables|/Game/Tsubasa/Core/Bluetilities/BP_BattleManager.BP_BattleManager_C|GetTeam2PWN_NPC _battlemanager_2))
  (bind _team1pwn_npc (Variables|/Game/Tsubasa/Core/Bluetilities/BP_BattleManager.BP_BattleManager_C|GetTeam1PWN_NPC _battlemanager_2))
  (bind _returnvalue_2 (select _returnvalue _team2pwn_npc _team1pwn_npc))
  (Utilities|FlowControl|Sequence
    (:then_0
      (LocalVariables|SetDistanceNearThreshold DistanceNearThreshold_In)
      (Utilities|IsValid _actorpossessingball
        (:Is%20Valid
          (LocalVariables|SetActorPossessingLocation (Transformation|GetActorLocation _actorpossessingball)))
        (:Is%20Not%20Valid
          (Development|PrintString "Hello"))))
    (:then_1
      (for _index (range 0 (- (Utilities|Array|Length _returnvalue_2) 1))
        (bind _output_get (LocalVariables|SetDistance (Math|Vector|Distance(Vector) (Transformation|GetActorLocation (Utilities|Array|Get(acopy) _returnvalue_2 _index)) (LocalVariables|GetActorPossessingLocation))))
        (if (<= _output_get (LocalVariables|GetDistanceNearThreshold))
          (return (Utilities|Array|Get(acopy) _returnvalue_2 _index))))
      (return 0))))

(fn ForceStartNPCBT
  (bind _aicontrollerreference (Variables|Default|GetAIControllerReference)
    (:then
      (Default|StopBT _aicontrollerreference)
      (Default|RunNPCBT _aicontrollerreference)
      (Variables|Default|SetbPlayerTurn false))
    (:else)))

(fn ForceStartPlayerTurnBT
  (bind _aicontrollerreference (Variables|Default|GetAIControllerReference)
    (:then
      (Default|StopBT _aicontrollerreference)
      (Default|RunPlayerBT _aicontrollerreference)
      (Variables|Default|SetbPlayerTurn true))
    (:else
      (Development|PrintString "Invalid controller reference"))))

(fn TriggerAbility
  (params (ID :type Integer))
  (bind _playerproperties (Variables|Default|GetPlayerProperties))
  (bind (_playercountry _playerrole _playerframeid _playerabilities) (Utilities|Struct|BreakPlayerProperties _playerproperties))
  (bind _output (Utilities|Array|Get(acopy) _playerabilities ID))
  (bind (_abilityname _abilitylevel _attacktype _staminacost _iconid _triggersequence) (Utilities|Struct|BreakPlayerAbility _output))
  (Class|FootballCharacter|SubtractStamina _staminacost)
  (Variables|Default|SetCurrentAttackType _attacktype)
  (if _triggersequence
    (Default|StopBT (Variables|Default|GetAIControllerReference))
    (Default|ClashAbility (Variables|/Game/Tsubasa/Core/Bluetilities/BP_BattleManager.BP_BattleManager_C|GetSequenceManager (Variables|Default|GetBattleManager)) 0 _abilityname _playerrole)
    (else
      (CallFunction|ForceStartPlayerTurnBT))))

(fn TriggerFieldSkill
  (params (AttackType :type EAttackTypes%20Enum :default "Default"))
  (Variables|Default|SetCurrentAttackType AttackType)
  (CallFunction|ForceStartPlayerTurnBT)
  (Development|PrintString "TriggerFieldSkill"))

(fn StopBTifInactive
  (if (not (Variables|Default|GetbPlayerTurn))
    (bind _aicontrollerreference (Variables|Default|GetAIControllerReference)
      (:then
        (Default|StopBT _aicontrollerreference)
        (Development|PrintString (Utilities|String|Append "Froze: " (Utilities|GetDisplayName self))))
      (:else))))

(fn StartBT
  (bind _aicontrollerreference (Variables|Default|GetAIControllerReference)
    (:then
      (Default|RestartBT _aicontrollerreference)
      (Variables|Default|SetbPlayerTurn false)
      (Development|PrintString "Restarted the BT after a freeze."))
    (:else)))

(fn TeleporttoStartLocation
  (Transformation|Teleport self (Variables|Default|GetSpawnPosition) "0, 0, 0"))

(fn IsClosetoEnemy
  (params (PossibleEnemy :type Actor%20Object%20Reference) (MaxDistCheck :type Float%20%28single-precision%29))
  (bind _self self)
  (bind _aspwn_npc (Utilities|Casting|CastToPWN_NPC PossibleEnemy)
    (:then
      (if (and (Math|Boolean|Equal(Boolean) (Class|FootballCharacter|IsTeam1 _aspwn_npc) (Class|FootballCharacter|IsTeam1 _self)) (<= (Class|KismetMathLibrary|VectorDistance2DSquared (Transformation|GetActorLocation _self) (Transformation|GetActorLocation _aspwn_npc)) (Math|Float|Square MaxDistCheck)))
        (return true)
        (else
          (return false))))
    (:CastFailed
      (return false))))

(fn IsEnemy
  (params (Actor :type Actor%20Object%20Reference))
  (bind _asfootball_character (Utilities|Casting|CastToFootballCharacter Actor))
  (if (Math|Boolean|Equal(Boolean) (Class|FootballCharacter|IsTeam1 _asfootball_character) (Class|FootballCharacter|IsTeam1 self))
    (return false)
    (else
      (return true))))

(fn UpdateBlackboardStates
  (params (BlackboardComponent :type Blackboard%20Component%20Object%20Reference))
  (AI|Components|Blackboard|SetValueasEnum BlackboardComponent (Utilities|Name|MakeLiteralName "State") (Variables|Default|GetPlayerStates))
  (AI|Components|Blackboard|SetValueasEnum BlackboardComponent (Utilities|Name|MakeLiteralName "AttackState") (Variables|Default|GetOffenseState)))

(fn PrintPlayerState
  (params (Screen :type Boolean) (Console :type Boolean))
  (Development|PrintString (Utilities|String|Append (Utilities|GetDisplayName self) " " (Utilities|String|EnumtoString (Variables|Default|GetPlayerStates))) Screen Console)
  (return))

(fn ActivateCooldown
  (params (Message :type String))
  (bind _returnvalue (|CallParentFunction Message))
  (if _returnvalue
    (CallFunction|ActivateCooldownTimer)
    (return _returnvalue)))