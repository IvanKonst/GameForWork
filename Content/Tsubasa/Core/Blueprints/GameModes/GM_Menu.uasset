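; GM_Menu is the menu game mode, which sets up player data and starts menu music on BeginPlay.
; It gets the player inventory from GI_TsubasaInstance and caches it for use in the following steps.
; It initializes the audio subsystem with field and home music arrays and the profile's saved volume, then plays home menu music.
; It also prints the profile's player name on screen.
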(event EventBeginPlay
  (bind _returnvalue (Subsystems|GetAudioSubsystem))
  (Utilities|FlowControl|Sequence
    (:then_0
      (bind _asgi_tsubasa_instance (Utilities|Casting|CastToGI_TsubasaInstance (Game|GetGameInstance)))
      (bind _output_get (Variables|Default|SetGameInstance _asgi_tsubasa_instance))
      (bind _playerinventory (Default|GetPlayerInventory _output_get))
      (Variables|Default|SetPlayerInventory _playerinventory))
    (:then_1
      (Class|AudioSubsystem|InitAudioSubsystem _returnvalue (Variables|Default|GetFieldMusic) (Variables|Default|GetHomeMusic) (Utilities|Struct|BreakGameSettings (Utilities|Struct|BreakFPlayerProfile (Utilities|Struct|BreakFPlayerInventory (Variables|Default|GetPlayerInventory)))))
      (Class|AudioSubsystem|PlayHomeMenuMusic _returnvalue))
    (:then_2
      (Development|PrintString (Utilities|String|ToString(Name) (.PlayerName (Utilities|Struct|BreakFPlayerProfile (Utilities|Struct|BreakFPlayerInventory (Variables|Default|GetPlayerInventory))))) true true "(R=0.682754,G=0.000000,B=1.000000,A=1.000000)"))))

(fn ConstructionScript)