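; Game mode for a stadium match that sets up the teams, runs the match clock and ends the round.
; On BeginPlay, if enabled, it caches player inventory, spawns the sequence manager for animations, hands it to the Battle Manager, spawns both teams and resets the score.
; It also starts optional audio, the team clothing color and anime-line media.
; A one-second looping timer triggers EndGame at the time limit, stopping behavior trees and broadcasting the end.
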(event Custom|ActivateMediaPlayerAnimeLines
  (Media|MediaPlayer|Play (Variables|Default|GetAnimeLinesMP) :!class /Script/MediaAssets.MediaPlayer))

(event EventBeginPlay
  (bind _returnvalue (Subsystems|GetAudioSubsystem))
  (if (Variables|Default|GetbBeginGame)
    (Utilities|FlowControl|Sequence
      (:then_0
        ;[1 1 1 1 22] Grab game instance and player inventory
        (bind _asgi_tsubasa_instance (Utilities|Casting|CastToGI_TsubasaInstance (Game|GetGameInstance)))
        (bind _output_get (Variables|Default|SetGameInstance _asgi_tsubasa_instance))
        (bind _playerinventory (Default|GetPlayerInventory _output_get))
        (Variables|Default|SetPlayerInventory _playerinventory))
      (:then_1
        ;[1 1 1 1 22] Initialize the timer and grab a BM reference, sequence manager
        (bind _returnvalue_2 (Utilities|Time|SetTimerbyFunctionName 0 "Timer" 1.0 true))
        (Variables|Default|SetGameTimerHandle _returnvalue_2)
        (bind _returnvalue_3 (Actor|GetActorOfClass "/Game/Tsubasa/Core/Bluetilities/BP_BattleManager.BP_BattleManager_C"))
        (Variables|Default|SetBattleManagerReference _returnvalue_3))
      (:then_2
        ;[1 1 1 1 22] Spawn and grab a reference to the sequence manager, responsible for the animations
        (bind _returnvalue_4 (Game|SpawnActorfromClass "/Game/Tsubasa/Core/Bluetilities/BP_SequenceManagerV2.BP_SequenceManagerV2_C" (Math|Transform|MakeTransform "0, 0, 0" "0, 0, 0" "1,1,1") "Undefined" 0 0))
        (bind _output_get_2 (Variables|Default|SetSequenceManagerV2 _returnvalue_4))
        (Variables|/Game/Tsubasa/Core/Bluetilities/BP_BattleManager.BP_BattleManager_C|SetSequenceManagerV2 (Variables|Default|GetBattleManagerReference) _output_get_2)
        ;;[1 1 1] Hardcode for the enemy color [ for now ]
        (Variables|/Game/Tsubasa/Core/Bluetilities/BP_SequenceManagerV2.BP_SequenceManagerV2_C|SetEnemyColor _output_get_2 "(R=0.068675,G=0.356404,B=1.000000,A=1.000000)")
        ;[1 1 1 1 22] Spawn the audio manager and run the field background music
        (if (Variables|Default|GetbEnableAudio)
          (Class|AudioSubsystem|InitAudioSubsystem _returnvalue (Variables|Default|GetFieldMusic) (Variables|Default|GetHomeMusic) (Utilities|Struct|BreakGameSettings (Utilities|Struct|BreakFPlayerProfile (Utilities|Struct|BreakFPlayerInventory (Variables|Default|GetPlayerInventory)))))
          (Class|AudioSubsystem|PlayFieldMusic _returnvalue)))
      (:then_3
        ;[1 1 1 1 22] Spawn teams
        (CallFunction|SpawnTeams)
        ;[1 1 1] Reset the score in the subsystem
        (Class|ScoreSubsystem|ResetScore (Subsystems|GetScoreSubsystem)))
      (:then_4
        ;[1 1 1 1 22] Set the color to the parameter collection
        (Rendering|Material|SetVectorParameterValue "/Game/CharacterFootballer/Materials/CharacterParameterCollection.CharacterParameterCollection" "ClothesColor" (.PlayerTeamColor (Utilities|Struct|BreakFPlayerProfile (Utilities|Struct|BreakFPlayerInventory (Variables|Default|GetPlayerInventory)))) :!class /Script/Engine.KismetMaterialLibrary))
      (:then_5
        (CallFunction|ActivateMediaPlayerAnimeLines)))))

(event Custom|Timer
  (CallFunction|CheckifEndGame)
  (Variables|Default|SetTimeSec (+ (Variables|Default|GetTimeSec) 1))
  (if (> (Variables|Default|GetTimeSec) 59)
    (Variables|Default|SetTimeMin (+ (Variables|Default|GetTimeMin) 1))
    (Variables|Default|SetTimeSec 0)))

(event Custom|EndGame
  (Variables|Default|SetbGameHasEnded true)
  (Default|CallStopBTDelegate (Variables|Default|GetBattleManagerReference))
  (Development|PrintString "EndGame" false)
  (Utilities|Time|ClearandInvalidateTimerbyHandle (Variables|Default|GetGameTimerHandle))
  (Default|CallEndGameDelegate))

(event Custom|StartBehaviourTree
  (bind _returnvalue (Actor|GetActorOfClass "/Game/Tsubasa/Core/Blueprints/PlayerControllers/AIC_NPC.AIC_NPC_C"))
  (Utilities|IsValid _returnvalue
    (:Is%20Valid
      (Default|CallStartBehaviourTree _returnvalue))))

(event Custom|CheckIfEndGame
  (if (>= (+ (Variables|Default|GetTimeSec) (* (Variables|Default|GetTimeMin) 60)) (Variables|Default|GetMaxSecondsRound))
    (if (not (Variables|Default|GetbGameHasEnded))
      (CallFunction|EndGame))))

(fn ConstructionScript)

(fn SpawnTeams
  (bind _battlemanagerreference (Variables|Default|GetBattleManagerReference)
    (:then
      (Default|SpawnTeam1 _battlemanagerreference false)
      (Default|SpawnTeam2Bots _battlemanagerreference true)
      (Class|BattleManager|DetermineStates _battlemanagerreference))
    (:else)))