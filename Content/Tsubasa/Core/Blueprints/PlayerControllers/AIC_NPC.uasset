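; AI controller for soccer NPCs that switches between the soccer player and player-turn behavior trees.
; On BeginPlay it sets up the NPC blackboard and binds start and stop events for both trees.
; Stopping halts logic and movement, while restarting or stopping the player tree reruns the soccer player tree.
; A helper function writes a new player state into the blackboard's State key.
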(event Custom|RunPlayerBT
  (AI|RunBehaviorTree (Variables|Default|GetBT_PlayerTurn))
  (Development|PrintString "PlayerTurnBT is running." false))

(event Custom|RunNPCBT
  (Utilities|IsValid (Variables|Default|GetBrainComponent)
    (:Is%20Valid
      (CallFunction|RestartBT)
      (Development|PrintString "RunNPCBT - RBT"))
    (:Is%20Not%20Valid
      (AI|RunBehaviorTree (Variables|Default|GetBT_SoccerPlayer))
      (Development|PrintString "NPCBT is running." false))))

(event Custom|StopBT
  (bind _braincomponent (Variables|Default|GetBrainComponent self)
    (:then
      (AI|Logic|StopLogic _braincomponent "")
      (Development|PrintString "StopBT" false)
      (AI|Navigation|StopMovement))
    (:else
      (Development|PrintString "BrainComponentInvalid(???)"))))

(event Custom|RestartBT
  (bind _braincomponent (Variables|Default|GetBrainComponent))
  (Utilities|IsValid _braincomponent
    (:Is%20Valid
      (AI|Logic|StopLogic _braincomponent ""))
    (:Is%20Not%20Valid
      _))
  (AI|Navigation|StopMovement)
  (AI|RunBehaviorTree (Variables|Default|GetBT_SoccerPlayer))
  (Development|PrintString "RestartBT"))

(event Custom|EvtNPCBT
  (CallFunction|RunNPCBT))

(event EventBeginPlay
  (Class|AIController|UseBlackboard "/Game/Tsubasa/Core/Blueprints/NPC/AIBT/BB_NPC.BB_NPC")
  (Utilities|FlowControl|Sequence
    (:then_0
      (EventDispatchers|BindEventtoStartBehaviourTree (delegate Custom|EvtNPCBT))
      (EventDispatchers|BindEventtoStartPlayerBehaviourTree (delegate Custom|RunPlayerBT)))
    (:then_1
      (EventDispatchers|BindEventtoStopBehaviourTree (delegate Custom|StopBT))
      (EventDispatchers|BindEventtoStopPlayerBehaviourTree (delegate Custom|RestartBT)))))

(fn ConstructionScript)

(fn UpdateStateOfBlackboard
  (params (New%20player%20state :type EPStates%20Enum :default "isBallInGoal"))
  (bind _self self)
  (bind _blackboard (Variables|Default|GetBlackboard _self))
  (Utilities|IsValid _blackboard
    (:Is%20Valid
      (AI|Components|Blackboard|SetValueasEnum _blackboard (Utilities|Name|MakeLiteralName "State") New%20player%20state))
    (:Is%20Not%20Valid
      (Development|PrintString "Invalid blackboard component in the AIC")))
  (return))