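; Player controller for the stadium match, mostly carrying debug tools for the player inventory and NPC abilities.
; BeginPlay caches the game instance's player inventory and enables game-and-UI input; debug keys print that inventory or append a default player.
; Number keys trigger abilities on the ball-holding NPC found by updatecurrentpawn, whose polling timer is disconnected.
; GetTargetPoints returns two tagged stadium corner markers.
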(event Custom|updatecurrentpawn
  ;[1 1 1] Create references
  (bind _outactors (Actor|GetAllActorsOfClass "/Game/Tsubasa/Core/Blueprints/Characters/PWN_NPC.PWN_NPC_C"))
  (for _array_element _outactors
    (if (Variables|/Script/AIProject.FootballCharacter|GetbHasBall _array_element)
      (Variables|Default|SetNPCDebugReference _array_element))))

(event EventBeginPlay
  (Utilities|FlowControl|Sequence
    (:then_0
      ;[1 1 1] Create references
      ;;[1 1 1] Get player inventory
      (bind _asgi_tsubasa_instance (Utilities|Casting|CastToGI_TsubasaInstance (Game|GetGameInstance)))
      (bind _output_get (Variables|Default|SetGameInstance _asgi_tsubasa_instance))
      (bind _playerinventory (Default|GetPlayerInventory _output_get))
      (Variables|Default|SetPlayerInventory _playerinventory))
    (:then_1
      (Input|SetInputModeGameandUI self 0 "DoNotLock" true))))

(event Input|KeyboardEvents|P
  (params (Key :type Key%20Structure))
  ;[1 1 1] print player info
  (:Pressed
    (for (_array_element _array_index) (.AllPlayers (Utilities|Struct|BreakFPlayerInventory (Variables|Default|GetPlayerInventory)))
      (Development|PrintString (Utilities|String|Append (Utilities|String|ToString(Name) (.Name (Utilities|Struct|BreakPlayerProperties _array_element))) (Utilities|String|ToString(Integer) _array_index)) true true "(R=0.108477,G=1.000000,B=0.110855,A=1.000000)"))))

(event Input|KeyboardEvents|K
  (params (Key :type Key%20Structure))
  (bind _returnvalue (Utilities|Name|MakeLiteralName "NewDefaultPlayer"))
  (bind _playerability (Utilities|Struct|MakePlayerAbility "DefaultAbName" 1 "KeepBall"))
  ;[1 1 1] print player info
  (:Pressed
    (Utilities|Array|Add (.AllPlayers (Utilities|Struct|BreakFPlayerInventory (Variables|Default|GetPlayerInventory))) (Utilities|Struct|MakePlayerProperties _returnvalue "Germany" "defender" "common" 1 "(Speed=100.000000,Attack=100.000000,Defence=100.000000,Stamina=100.000000)" 0 1e+02 -1 -1 -1 (Utilities|Array|MakeArray _playerability _playerability _playerability _playerability)))
    (Development|PrintString (Utilities|String|Append "Added to game save: " (Utilities|String|ToString(Name) _returnvalue)))
    (Default|UpdatePlayerInventory (Variables|Default|GetGameInstance) (Variables|Default|GetPlayerInventory))))

(event Input|KeyboardEvents|T
  (params (Key :type Key%20Structure))
  (:Pressed
    (Development|PrintString "Hello")))

(event Input|KeyboardEvents|1
  (params (Key :type Key%20Structure))
  (:Pressed
    (Default|TriggerAbility (Variables|Default|GetNPCDebugReference))))

(event Input|KeyboardEvents|2
  (params (Key :type Key%20Structure))
  (:Pressed
    (Default|TriggerAbility (Variables|Default|GetNPCDebugReference) 1)))

(event Input|KeyboardEvents|3
  (params (Key :type Key%20Structure))
  (:Pressed
    (Default|TriggerAbility (Variables|Default|GetNPCDebugReference) 2)))

(event Input|KeyboardEvents|4
  (params (Key :type Key%20Structure))
  (:Pressed
    (Default|TriggerAbility (Variables|Default|GetNPCDebugReference) 3)))

(fn ConstructionScript)

(fn GetTargetPoints
  (bind _targetpointsstadium (Variables|Default|GetTargetPointsStadium))
  (Utilities|FlowControl|Sequence
    (:then_0
      (bind _outactors (Actor|GetAllActorsOfClasswithTag "/Script/Engine.TargetPoint" "topright"))
      (bind _astarget_point (Utilities|Casting|CastToTargetPoint (Utilities|Array|Get(acopy) _outactors)))
      (Utilities|Array|Add _targetpointsstadium _astarget_point))
    (:then_1
      (bind _outactors_2 (Actor|GetAllActorsOfClasswithTag "/Script/Engine.TargetPoint" "botleft"))
      (bind _astarget_point_2 (Utilities|Casting|CastToTargetPoint (Utilities|Array|Get(acopy) _outactors_2)))
      (Utilities|Array|Add _targetpointsstadium _astarget_point_2)
      (return _targetpointsstadium))))