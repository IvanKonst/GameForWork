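; Behavior Tree task that looks around the controlled pawn for an NPC location to store in the Blackboard.
; It runs a sphere overlap for static and dynamic world objects within Radius, with a loop meant to break on PWN_NPC.
; The current array element's location goes to VecKey without any distance comparison, despite the asset's name.
; Success follows the overlap result, with a debug sphere and printout.
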(event EventReceiveExecuteAI
  (params (OwnerController :type AI%20Controller%20Object%20Reference) (ControlledPawn :type Pawn%20Object%20Reference))
  (bind _returnvalue (Transformation|GetActorLocation ControlledPawn))
  (bind _radius (Variables|Default|GetRadius))
  (Rendering|Debug|DrawDebugSphere _returnvalue _radius 12 "(R=1.000000,G=1.000000,B=1.000000,A=1.000000)" 2.0 1.0)
  (bind (_outactors _returnvalue_2) (Collision|SphereOverlapActors _returnvalue _radius (Utilities|Array|MakeArray "ObjectTypeQuery1" "ObjectTypeQuery2") 0))
  (if (== (stale _array_element) "/Game/Tsubasa/Core/Blueprints/Characters/PWN_NPC.PWN_NPC")
    (goto _label Break)
    (else
      (bind _array_element (Utilities|Array|ForEachLoopwithBreak _outactors :!label _label)
        (:Completed
          (AI|BehaviorTree|SetBlackboardValueasVector (Variables|Default|GetVecKey) (Transformation|GetActorLocation _array_element))
          (Development|PrintString (Utilities|String|ToString(Boolean) _returnvalue_2))
          (AI|BehaviorTree|FinishExecute _returnvalue_2))))))